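; PostGenerator actor that spawns and tracks Post actors from the top center of the player's camera view.
; On BeginPlay it moves to the side-scroller character's CamTopCenter, then spawns the first Post at its own transform.
; Each new Post becomes CurrentPost and is added to the Posts array.
; Events forward text additions to CurrentPost or submit it, with submission immediately spawning the next Post.
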(event Custom|CreateNewPost
  (bind _returnvalue (Game|SpawnActorfromClass "/Game/Blueprints/Post.Post_C" (Transformation|GetWorldTransform (Variables|Default|GetScene)) "AlwaysSpawn" 0 0))
  (bind _output_get (Variables|Default|SetcurrentPost _returnvalue))
  (Utilities|Array|Add (Variables|Default|GetPosts) _output_get))

(event Custom|SubmitCurrentPost
  (Default|Submit (Variables|Default|GetcurrentPost))
  (CallFunction|CreateNewPost))

(event Custom|AddTextToCurrPost
  (Default|OnTextAdded (Variables|Default|GetcurrentPost)))

(event EventBeginPlay
  (Utilities|FlowControl|Sequence
    (:then_0
      ;[1 1 1] Position itself
      (bind _as2dside_scroller_character (Utilities|Casting|CastTo2DSideScrollerCharacter (Game|GetPlayerCharacter 0)))
      (Transformation|SetWorldLocation (Variables|Default|GetScene) (Variables|/Game/Blueprints/2DSideScrollerCharacter.2DSideScrollerCharacter_C|GetcamTopCenter _as2dside_scroller_character) false false))
    (:then_1
      (CallFunction|CreateNewPost))))

(event Collision|EventActorBeginOverlap
  (params (OtherActor :type Actor%20Object%20Reference)))

(event EventTick
  (params (DeltaSeconds :type Float%20%28single-precision%29)))

(fn ConstructionScript)