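; Post actor with a Paper2D sprite that reacts to text being added and to being submitted.
; Added text triggers a timeline-driven shake that randomly offsets the sprite in X and Z within ShakeAmount, then resets it to its origin.
; Submit plays the same shake and sets IsSubmitted, after which Tick slides the Scene component down along local Z by a fixed, frame-rate-dependent step.
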(event Custom|OnTextAdded
  (CallFunction|Shake))

(event Custom|Shake
  (bind _shakeamount (Variables|Default|GetshakeAmount))
  (bind _returnvalue (* -1 _shakeamount))
  (Timeline|ShakeTimeline PlayFromStart
    (:Update
      (Transformation|SetRelativeLocation (Variables|Default|GetPaperSprite) (Math|Vector|MakeVector (Math|Random|RandomFloatinRange _returnvalue _shakeamount) 0.0 (Math|Random|RandomFloatinRange _returnvalue _shakeamount)) false false))
    (:Finished
      (Transformation|SetRelativeLocation (Variables|Default|GetPaperSprite) "0, 0, 0" false false))))

(event Custom|Submit
  (CallFunction|Shake)
  (Variables|Default|SetisSubmitted true))

(event EventBeginPlay)

(event Collision|EventActorBeginOverlap
  (params (OtherActor :type Actor%20Object%20Reference)))

(event EventTick
  (params (DeltaSeconds :type Float%20%28single-precision%29))
  (Utilities|FlowControl|Sequence
    (:then_0
      ;[1 1 1] Movement
      (if (Variables|Default|GetisSubmitted)
        (Transformation|AddLocalOffset (Variables|Default|GetScene) "0, 0,-5.000000" false false)))))

(fn ConstructionScript)